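; Blueprint function library of shared transform helpers that turn an actor to face a world location.
; LookAtTarget and RotateTowardsLocation do the same work: each computes a look-at rotation from the owner's location to the given point and applies it with SetActorRotation.
; The rotation snaps in a single call on all axes returned by the look-at, with no interpolation and no physics teleport.
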(fn `LookAtTarget`
  (params (owner :type "Actor Object Reference") (Target :type "Vector Structure (by ref)"))
  (locals (TargetLookAt :type "Actor Object Reference"))
  (bind _output_get (set `local.TargetLookAt` owner))
  (`Actor.K2_SetActorRotation` _output_get (`KismetMathLibrary.FindLookAtRotation` (`Actor.K2_GetActorLocation` owner) Target) false)
  (return))

(fn `RotateTowardsLocation`
  (params (owner :type "Actor Object Reference") (Location :type "Vector Structure"))
  (locals (CapsuleComponent :type "CapsuleComponent Object Reference") (NewLocation :type "Vector Structure"))
  (`Actor.K2_SetActorRotation` owner (`KismetMathLibrary.FindLookAtRotation` (`Actor.K2_GetActorLocation` owner) Location) false)
  (return))