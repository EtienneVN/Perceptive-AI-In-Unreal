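; BP_Char_Guard is a guard NPC character that carries a spawned weapon and exposes its death status and patrol route.
; BeginPlay saves the start transform and attaches the weapon to a mesh socket.
; State changes are forwarded to the AnimInstance, and movement speed is set per state.
; On first death it ragdolls, then after a delay resets health and teleports to its start, without undoing the ragdoll.
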(event `self.ReceiveBeginPlay`
  (set `self.GetInitLocation` (`self.GetTransform` self))
  (bind _returnvalue (`|SpawnActorFromClass` (`self.WeaponClass`) (`/Game/Blueprints/Shared/BPL_Library.IdentityTransform`) "AlwaysSpawn" "OverrideRootScale" self self))
  (bind _output_get (set `self.Weapon` _returnvalue))
  (`self.K2_AttachToComponent` _output_get (`self.Mesh`) "WeaponSocket" "SnapToTarget" "SnapToTarget" "SnapToTarget" true))

(event `self.HealthComponent.OnDamageTaken`)

(event `self.HealthComponent.OnDeath`
  (bind _healthcomponent (`self.HealthComponent`))
  (`/Engine/EditorBlueprintResources/StandardMacros.DoOnce` false
    (:`Completed`
      (`PrimitiveComponent.SetCollisionProfileName` (`self.Mesh`) "Ragdoll" true)
      (`SkeletalMeshComponent.SetAllBodiesSimulatePhysics` (`self.Mesh`) true)
      (`PrimitiveComponent.WakeAllRigidBodies` (`self.Mesh`))
      (`PrimitiveComponent.SetCollisionEnabled` (`self.CapsuleComponent`) "NoCollision")
      (`KismetSystemLibrary.PrintString` (`KismetStringLibrary.Concat_StrStr` (`KismetSystemLibrary.GetDisplayName` self) "Died!"))
      (`KismetSystemLibrary.Delay` 3.0)
      (set `/Game/Blueprints/Shared/HealthComponent.Health` 50.0 _healthcomponent)
      (set `self.HealthComponent` _healthcomponent)
      (`self.K2_SetActorLocationAndRotation` (.location (`self.GetInitLocation`)) (.rotation (`self.GetInitLocation`)) false true))))

(event `/Game/Blueprints/Shared/BPI_AI_Helper.NotifyStateChange`
  (params (NewState :type "/Game/AI/Enums/NPC_State Enum" :default "NewEnumerator0"))
  ;[1 1 1] On State Changed
  (message `/Game/Blueprints/Shared/BPI_AI_Helper.NotifyStateChange` (`SkeletalMeshComponent.GetAnimInstance` (`self.Mesh`)) NewState))

(event `/Game/Blueprints/Shared/BPI_AI_Helper.ModifyMovementSpeed`
  (params (State :type "/Game/AI/Enums/NPC_State Enum" :default "NewEnumerator0"))
  (set `CharacterMovementComponent.MaxWalkSpeed` (select `/Game/AI/Enums/NPC_State` State :`NewEnumerator0` 160.0 :`NewEnumerator1` 160.0 :`NewEnumerator2` 400.0 :`NewEnumerator3` 600.0 :!type "Float (single-precision)") (`self.CharacterMovement`)))

(fn `GetIsDead`
  (returns (Dead :type Boolean))
  (return (`/Game/Blueprints/Shared/HealthComponent.isDead` (`self.HealthComponent`))))

(fn `GetPatrolRoute`
  (returns (PatrolRoute :type "/Game/Blueprints/NPC/PatrolRoute Object Reference"))
  (return (`self.MyPatrolPath`)))

(fn `GetTeamID`)

(fn `UserConstructionScript`)