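; Patrol route Blueprint that supplies waypoints as world positions, using the child components of PatrolPath as points.
; GetNextPointAsWorldPosition returns a randomly indexed child's location, ignoring PatrolIndex and making a stray ArraySet on the children array.
; The incrementPatrolPath event separately advances PatrolIndex, wrapping at the child count.
; GetIsDead, GetTeamID and GetPatrolRoute are stubs returning false or nothing, and BeginPlay, overlap and Tick are unused.
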(event `increment PatrolPath`
  (bind _patrolindex (`self.PatrolIndex`))
  (bind (_indexofmaxvalue _maxvalue) (`KismetMathLibrary.MaxOfIntArray` (`|MakeArray` (`SceneComponent.GetNumChildrenComponents` (`self.PatrolPath`)))))
  (if (< _patrolindex _maxvalue)
    (set `self.PatrolIndex` (mod (+ _patrolindex 1) _maxvalue))
    (else
      (set `self.PatrolIndex` 0))))

(fn `GetIsDead`
  (returns (Dead :type Boolean))
  (return false))

(fn `GetNextPointAsWorldPosition`
  (returns (ReturnValue :type "Vector Structure"))
  (bind _patrolpath (`self.PatrolPath`))
  (bind _children (`SceneComponent.GetChildrenComponents` _patrolpath true))
  (bind _returnvalue (`KismetMathLibrary.RandomInteger` (`KismetArrayLibrary.Array_Length` _children)))
  (`KismetArrayLibrary.Array_Set` _children _returnvalue null true)
  (return (`SceneComponent.K2_GetComponentLocation` (`SceneComponent.GetChildComponent` _patrolpath _returnvalue))))

(fn `GetPatrolRoute`
  (returns (PatrolRoute :type "/Game/Blueprints/NPC/PatrolRoute Object Reference"))
  (return null))

(fn `GetTeamID`
  (returns (isPlayer :type Boolean))
  (return false))

(fn `UserConstructionScript`)