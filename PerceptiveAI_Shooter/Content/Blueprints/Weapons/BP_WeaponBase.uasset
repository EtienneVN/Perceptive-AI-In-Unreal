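; BP_WeaponBase is a weapon Blueprint, apparently a base class, that fires a round when fire is requested.
; FireRound spawns a BulletClass actor at the muzzle, plays a fire sound and runs a debug-drawn Visibility line trace.
; The trace end adds WeaponRange to the forward vector instead of scaling it.
; Point damage and AI damage-sense reporting nodes exist but are disconnected, so trace hits do nothing.
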(event `OnFireRequested`
  (`self.FireRound`))

(event `FireRound`
  (bind _returnvalue (`SceneComponent.K2_GetComponentLocation` (`self.MuzzlePosition`)))
  (`|SpawnActorFromClass` (`self.BulletClass`) (`SceneComponent.K2_GetComponentToWorld` (`self.MuzzlePosition`)) "AlwaysSpawn" "OverrideRootScale" null null)
  (`GameplayStatics.PlaySoundAtLocation` "/Game/FirstPerson/Audio/FirstPersonTemplateWeaponFire02.FirstPersonTemplateWeaponFire02" _returnvalue (struct) 1.0 1.0 0.0 null null null)
  (bind (_outhit _returnvalue_2) (`KismetSystemLibrary.LineTraceSingle` :`Start` _returnvalue :`End` (+ _returnvalue (+ (`SceneComponent.GetForwardVector` (`self.MuzzlePosition`)) (`self.WeaponRange`))) :`TraceChannel` "TraceTypeQuery1" :`DrawDebugType` "ForDuration"))
  (if _returnvalue_2
    _))

(fn `UserConstructionScript`)